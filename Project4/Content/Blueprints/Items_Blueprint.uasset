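; Items_Blueprint is an item actor with name, weight and durability that can trigger a customer spawn by key press.
; The construction script sets weight and durability from the item's name, with one case for Apple and a fallback for all others.
; It enables input from player 0 on BeginPlay; pressing F while Controlled prints a debug message, calls SpawnNext on its Customer reference and clears Controlled.
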(event EventBeginPlay
  (Input|EnableInput (Game|GetPlayerController 0)))

(event Collision|EventActorBeginOverlap
  (params (OtherActor :type Actor%20Object%20Reference)))

(event EventTick
  (params (DeltaSeconds :type Float%20%28single-precision%29)))

(event Input|KeyboardEvents|F
  (params (Key :type Key%20Structure))
  (:Pressed
    (if (Variables|Default|GetControlled)
      (Development|PrintString "Hello")
      (Default|SpawnNext (Variables|Default|GetCustomer))
      (Variables|Default|SetControlled false))))

(fn ConstructionScript
  (if (Utilities|Enum|Equal(Enum) (Variables|Default|GetName) (Utilities|String|MakeLiteralString "Apple"))
    (Variables|Default|SetWeight 5)
    (Variables|Default|SetDurability 10)
    (else
      (Variables|Default|SetWeight 4)
      (Variables|Default|SetDurability 8))))