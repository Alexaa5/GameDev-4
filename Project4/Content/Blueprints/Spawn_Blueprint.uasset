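; Spawner Blueprint that creates Items_Blueprint actors on request, up to an AmountOfItems cap.
; SpawnNext prints the ItemArray count and, while it is below the cap, spawns one item at SpawnLoc and adds it to the array.
; Each item receives the spawner as its Customer, a Controlled flag and a hardcoded Apple name, which a to-do marks for replacement by a set of strings.
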(event Custom|SpawnNext
  (bind _itemarray (Variables|Default|GetitemArray))
  (bind _returnvalue (Utilities|Array|Length _itemarray))
  (Development|PrintString (Utilities|String|ToString(Integer) _returnvalue))
  (Math|Integer|CompareInt _returnvalue (Variables|Default|GetAmountOfItems)
    (:<
      (bind _returnvalue_2 (Game|SpawnActorfromClass "/Game/Items_Blueprint.Items_Blueprint_C" (Math|Transform|MakeTransform (Variables|Default|GetSpawnLoc)) "Undefined" 0 "\"Apple\"" self true 0)) ; To do: change name so that it spawns an element from a set of strings
      (Utilities|Array|Add (Variables|Default|GetitemArray) _returnvalue_2))))

(event EventBeginPlay)

(event Collision|EventActorBeginOverlap
  (params (OtherActor :type Actor%20Object%20Reference)))

(event EventTick
  (params (DeltaSeconds :type Float%20%28single-precision%29)))

(fn ConstructionScript)